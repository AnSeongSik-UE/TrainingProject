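; BP_Rect is an actor that moves its Cube component around a looping square path in the local XZ plane.
; A Direction enum acts as a four-state machine on Tick, cycling Right, Up, Left, Down whenever the cube passes a bound.
; A Toggle flag flips each frame so the cube steps only every other tick, by a fixed amount independent of delta time.
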(event `self.ReceiveTick`
  (params (DeltaSeconds :type "Float (single-precision)"))
  ; 토글
  (bind _output_get (set `self.bToggle` (not (`self.bToggle`))))
  (if _output_get
    (switch `/Game/AnSik/EN_Direction` (`self.Direction`)
      (:`NewEnumerator0`
        (bind _output_get_2 (set `self.DirectionX` (+ (`self.DirectionX`) 10.0)))
        (`SceneComponent.K2_SetRelativeLocation` (`self.Cube`) (`KismetMathLibrary.MakeVector` _output_get_2 0.0 (`self.DirectionZ`)) false false)
        (if (> (`self.DirectionX`) 500.0)
          (set `self.Direction` "NewEnumerator1")))
      (:`NewEnumerator1`
        (bind _output_get_3 (set `self.DirectionZ` (+ (`self.DirectionZ`) 10.0)))
        (`SceneComponent.K2_SetRelativeLocation` (`self.Cube`) (`KismetMathLibrary.MakeVector` (`self.DirectionX`) 0.0 _output_get_3) false false)
        (if (> (`self.DirectionZ`) 500.0)
          (set `self.Direction` "NewEnumerator2")))
      (:`NewEnumerator2`
        (bind _output_get_4 (set `self.DirectionX` (+ (`self.DirectionX`) -10.0)))
        (`SceneComponent.K2_SetRelativeLocation` (`self.Cube`) (`KismetMathLibrary.MakeVector` _output_get_4 0.0 (`self.DirectionZ`)) false false)
        (if (< (`self.DirectionX`) 0.0)
          (set `self.Direction` "NewEnumerator3")))
      (:`NewEnumerator3`
        (bind _output_get_5 (set `self.DirectionZ` (+ (`self.DirectionZ`) -10.0)))
        (`SceneComponent.K2_SetRelativeLocation` (`self.Cube`) (`KismetMathLibrary.MakeVector` (`self.DirectionX`) 0.0 _output_get_5) false false)
        (if (< (`self.DirectionZ`) 0.0)
          (set `self.Direction` "NewEnumerator0"))))))

(fn `UserConstructionScript`)