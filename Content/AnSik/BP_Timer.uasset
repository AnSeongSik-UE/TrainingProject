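; BP_Timer is a timer actor that shows elapsed time as zero-padded minutes:seconds on a TextRender.
; Tick flips a toggle and, only on every other frame, adds that frame's DeltaSeconds to a running total, so it counts roughly half of real time.
; It prints the total, converts minutes and seconds through the FloatTo00 helper, and sets the text after each conversion.
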(event `self.ReceiveTick`
  (params (DeltaSeconds :type "Float (single-precision)"))
  (bind _output_get (set `self.bToggle` (not (`self.bToggle`))))
  (if _output_get
    (bind _output_get_2 (set `self.TotalDeltaSeconds` (+ DeltaSeconds (`self.TotalDeltaSeconds`))))
    (`KismetSystemLibrary.PrintString` (`KismetStringLibrary.Conv_DoubleToString` _output_get_2))
    (`|ExecutionSequence`
      (:`then_0`
        (bind _str00 (`self.FloatTo00` (/ _output_get_2 60.0))))
      (:`then_1`
        (bind _str00_2 (`self.FloatTo00` (mod _output_get_2 60.0)))))
    (`TextRenderComponent.K2_SetText` (`self.TextRender`) (`KismetTextLibrary.Conv_StringToText` (`KismetStringLibrary.Concat_StrStr` _str00 ":" _str00_2)))))

(fn `FloatTo00`
  (params (Value :type "Float (double-precision)"))
  (returns (Str00 :type String))
  (bind _returnvalue (`KismetMathLibrary.FFloor` Value))
  (if (> _returnvalue 9)
    (return (`KismetStringLibrary.Conv_IntToString` _returnvalue))
    (else
      (return (`KismetStringLibrary.Concat_StrStr` "0" (`KismetStringLibrary.Conv_IntToString` _returnvalue))))))

(fn `UserConstructionScript`)