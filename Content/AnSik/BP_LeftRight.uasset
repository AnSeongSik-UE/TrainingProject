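; BP_LeftRight moves a Cube along local X each Tick, apparently intended as a left-right shuttle between two X limits.
; After the move, a Sequence calls DirectionPlus and DirectionSubtract, which test relative X against the upper and lower limits.
; Both calls lead to a shared step that negates DeltaTransformLocationX.
; The limit branches show empty bodies, with no visible gating of that reversal.
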(event `self.ReceiveTick`
  (params (DeltaSeconds :type "Float (single-precision)"))
  ; 큐브이동
  (`SceneComponent.K2_AddLocalTransform` (`self.Cube`) (`KismetMathLibrary.MakeTransform` (`KismetMathLibrary.MakeVector` (`self.DeltaTransformLocationX`))) false false)
  (`|ExecutionSequence`
    (:`then_0`
      (`self.DirectionPlus`))
    (:`then_1`
      (`self.DirectionSubtract`)))
  ; 방향전환
  (set `self.DeltaTransformLocationX` (* (`self.DeltaTransformLocationX`) -1.0)))

(fn `DirectionPlus`
  (bind _relativelocation_x (`KismetMathLibrary.BreakVector` (`SceneComponent.RelativeLocation` (`self.Cube`))))
  (if (> _relativelocation_x 500.0)
    _))

(fn `DirectionSubtract`
  (bind _relativelocation_x (`KismetMathLibrary.BreakVector` (`SceneComponent.RelativeLocation` (`self.Cube`))))
  (if (< _relativelocation_x 0.0)
    _))

(fn `UserConstructionScript`)